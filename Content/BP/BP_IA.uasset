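; BP_IA is an AI enemy that chases the player and explodes on contact, costing a life.
; When Pawn Sensing sees a BP_Character, AI MoveTo moves the enemy toward it.
; On a successful move, the enemy destroys itself, spawns explosion particles and sound at player 0's location, and decrements Vidas in BP_Gamemode.
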(event `self.PawnSensing.OnSeePawn`
  (params (Pawn :type "Pawn Object Reference"))
  (bind _returnvalue (`self.K2_GetActorLocation` (`GameplayStatics.GetPlayerCharacter` 0)))
  (bind _asbp_character (cast `/Game/BP/BP_Character` Pawn))
  (`|AIMoveTo` self (0.0 0.0 0.0) _asbp_character
    (:`OnSuccess`
      (`self.K2_DestroyActor`)
      (`GameplayStatics.SpawnEmitterAtLocation` "/Game/StarterContent/Particles/P_Explosion.P_Explosion" _returnvalue)
      (`GameplayStatics.PlaySoundAtLocation` "/Game/StarterContent/Audio/Explosion_Cue.Explosion_Cue" _returnvalue (struct) 1.0 1.0 0.0 null null null)
      (bind _asbp_gamemode (cast `/Game/BP/BP_GameMode` (`GameplayStatics.GetGameMode`)))
      (set `/Game/BP/BP_GameMode.Vidas` (- (`/Game/BP/BP_GameMode.Vidas` _asbp_gamemode) 1) _asbp_gamemode))))

(fn `UserConstructionScript`)