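; BP_Llave is a key pickup that the player collects with the Accion input.
; A timeline started on BeginPlay drives the Sphere's relative Z location.
; The Box overlap enables or disables the actor's input as BP_Character enters or leaves, toggling the TextRender each time.
; Pressing Accion sets Llave on BP_Gamemode, then destroys the actor if the player character is a BP_Character.
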(event `self.ReceiveBeginPlay`
  (bind (_direction _newtrack_0) (`Timeline|Timeline_0`)
    (:`Update`
      (`SceneComponent.K2_SetRelativeLocation` (`self.Sphere`) (`KismetMathLibrary.MakeVector` 0.0 0.0 _newtrack_0) false false))))

(event `InputAction|Accion`
  (params (Key :type "Key Structure"))
  (:`Pressed`
    (bind _asbp_gamemode (cast `/Game/BP/BP_GameMode` (`GameplayStatics.GetGameMode`)))
    (set `/Game/BP/BP_GameMode.Llave?` true _asbp_gamemode)
    (cast `/Game/BP/BP_Character` (`GameplayStatics.GetPlayerCharacter` 0))
    (`self.K2_DestroyActor`)))

(event `self.Box.OnComponentBeginOverlap`
  (params (OverlappedComponent :type "PrimitiveComponent Object Reference") (OtherActor :type "Actor Object Reference") (OtherComp :type "PrimitiveComponent Object Reference") (OtherBodyIndex :type Integer) (bFromSweep :type Boolean) (SweepResult :type "HitResult Structure (by ref)"))
  (cast `/Game/BP/BP_Character` OtherActor)
  (`self.EnableInput` (`GameplayStatics.GetPlayerController` 0))
  (`SceneComponent.ToggleVisibility` (`self.TextRender`) false))

(event `self.Box.OnComponentEndOverlap`
  (params (OverlappedComponent :type "PrimitiveComponent Object Reference") (OtherActor :type "Actor Object Reference") (OtherComp :type "PrimitiveComponent Object Reference") (OtherBodyIndex :type Integer))
  (cast `/Game/BP/BP_Character` OtherActor)
  (`self.DisableInput` (`GameplayStatics.GetPlayerController` 0))
  (`SceneComponent.ToggleVisibility` (`self.TextRender`) false))

(fn `UserConstructionScript`)