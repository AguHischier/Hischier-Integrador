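; BP_GameMode is the game mode that tracks coins, lives, death and a game timer.
; BeginPlay calls EmpezarJuego, which zeroes Tiempo and starts a looping one-second timer on Reloj, an empty event.
; RecolectarMonedas counts coins and grants a life when the bonus counter equals ten and lives are below three.
; Tick polls for zero lives, flags death and opens the level named by Nivel after a delay.
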(event `self.ReceiveBeginPlay`
  (`self.EmpezarJuego`))

(event `Reloj`)

(event `self.ReceiveTick`
  (params (DeltaSeconds :type "Float (single-precision)"))
  (if (== (`self.Vidas`) 0)
    (set `self.Murio` true)
    (`KismetSystemLibrary.Delay` 3.0)
    (`GameplayStatics.OpenLevel` (`KismetStringLibrary.Conv_StringToName` (`self.Nivel`)))))

(fn `RecolectarMonedas`
  (bind _returnvalue (== (`self.MonedasVida`) 10))
  (set `self.Monedas` (+ (`self.Monedas`) 1))
  (set `self.MonedasVida` (+ (`self.MonedasVida`) 1))
  (if (and (< (`self.Vidas`) 3) _returnvalue)
    (if _returnvalue
      (set `self.MonedasVida` 0)
      (set `self.Vidas` (+ (`self.Vidas`) 1))
      (else
        (set `self.MonedasVida` 0)))))

(fn `UserConstructionScript`)