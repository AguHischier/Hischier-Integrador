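; BP_Puerta is a locked door actor that the player opens with a key to leave the level.
; Overlapping the Cubo volume with BP_Character toggles the text render and enables the Accion input, which is disabled again on exit.
; Accion checks the Llave flag in BP_Gamemode, either prompting for the key or calling AbrirPuerta after a delay.
; AbrirPuerta spawns BP_Portal, opens Menu whatever NivelNumero is, and destroys the door.
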(event `InputAction|Accion`
  (params (Key :type "Key Structure"))
  (:`Pressed`
    (bind _asbp_gamemode (cast `/Game/BP/BP_GameMode` (`GameplayStatics.GetGameMode`)))
    (if (`/Game/BP/BP_GameMode.Llave?` _asbp_gamemode)
      (`KismetSystemLibrary.Delay` 1.0)
      (`self.Abrir Puerta`)
      (else
        (`KismetSystemLibrary.PrintString` "Encuentra la llave")))))

(event `self.Cubo.OnComponentBeginOverlap`
  (params (OverlappedComponent :type "PrimitiveComponent Object Reference") (OtherActor :type "Actor Object Reference") (OtherComp :type "PrimitiveComponent Object Reference") (OtherBodyIndex :type Integer) (bFromSweep :type Boolean) (SweepResult :type "HitResult Structure (by ref)"))
  (cast `/Game/BP/BP_Character` OtherActor)
  (`self.EnableInput` (`GameplayStatics.GetPlayerController` 0))
  (`SceneComponent.ToggleVisibility` (`self.TextRender`) false))

(event `self.Cubo.OnComponentEndOverlap`
  (params (OverlappedComponent :type "PrimitiveComponent Object Reference") (OtherActor :type "Actor Object Reference") (OtherComp :type "PrimitiveComponent Object Reference") (OtherBodyIndex :type Integer))
  (cast `/Game/BP/BP_Character` OtherActor)
  (`self.DisableInput` (`GameplayStatics.GetPlayerController` 0))
  (`SceneComponent.ToggleVisibility` (`self.TextRender`) false))

(fn `Abrir Puerta`
  (bind _asbp_gamemode (cast `/Game/BP/BP_GameMode` (`GameplayStatics.GetGameMode`)))
  (`|SpawnActorFromClass` "/Game/BP/BP_Portal.BP_Portal_C" (`KismetMathLibrary.Conv_VectorToTransform` (`SceneComponent.K2_GetComponentLocation` (`self.Cube`))) "AlwaysSpawn" "OverrideRootScale" null null)
  (if (== (`/Game/BP/BP_GameMode.Nivel_Numero` _asbp_gamemode) 3)
    _
    (else
      _))
  (`GameplayStatics.OpenLevel` "Menu")
  (`self.K2_DestroyActor`))

(fn `UserConstructionScript`)