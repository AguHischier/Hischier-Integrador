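; BP_Hongo is a mushroom pickup that temporarily boosts the jump height of the BP_Character that overlaps its Cube.
; On overlap it hides itself and raises the character's AlturaSalto, then after a ten-second delay restores a lower fixed value and reappears.
; Hiding leaves collision untouched, and an unconnected SpawnActor node for another BP_Hongo never runs.
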(event `self.ReceiveBeginPlay`
  (bind _cube (`self.Cube`))
  (`SceneComponent.K2_SetRelativeLocation` _cube (`SceneComponent.RelativeLocation` _cube) false false))

(event `self.Cube.OnComponentBeginOverlap`
  (params (OverlappedComponent :type "PrimitiveComponent Object Reference") (OtherActor :type "Actor Object Reference") (OtherComp :type "PrimitiveComponent Object Reference") (OtherBodyIndex :type Integer) (bFromSweep :type Boolean) (SweepResult :type "HitResult Structure (by ref)"))
  (bind _asbp_character (cast `/Game/BP/BP_Character` OtherActor))
  (`self.SetActorHiddenInGame` true)
  (set `/Game/BP/BP_Character.AlturaSalto` (0.0 0.0 3100.0) _asbp_character)
  (`KismetSystemLibrary.Delay` 10.0)
  (set `/Game/BP/BP_Character.AlturaSalto` (0.0 0.0 800.0) _asbp_character)
  (`self.SetActorHiddenInGame` false))

(fn `UserConstructionScript`)