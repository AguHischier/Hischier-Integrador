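; BP_Pelota is a player-controlled physics ball that rolls along one axis and jumps.
; The MoveRight axis, scaled by Velocidad, applies an angular impulse to the Sphere around X, so movement comes from spin.
; Jump adds an upward velocity-change impulse and clears PuedeSaltar, blocking further jumps.
; Sphere hits on actors tagged "Piso" (floor) set PuedeSaltar again.
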(event `InputAxis|MoveRight`
  (params (AxisValue :type "Float (single-precision)"))
  (`PrimitiveComponent.AddAngularImpulseInDegrees` (`self.Sphere`) (`KismetMathLibrary.MakeVector` (* AxisValue (`self.Velocidad`))) "None" true))

(event `InputAction|Jump`
  (params (Key :type "Key Structure"))
  (:`Pressed`
    (if (`self.PuedeSaltar`)
      (`PrimitiveComponent.AddImpulse` (`self.Sphere`) (0.0 0.0 500.0) "None" true)
      (set `self.PuedeSaltar` false))))

(event `self.Sphere.OnComponentHit`
  (params (HitComponent :type "PrimitiveComponent Object Reference") (OtherActor :type "Actor Object Reference") (OtherComp :type "PrimitiveComponent Object Reference") (NormalImpulse :type "Vector Structure") (Hit :type "HitResult Structure (by ref)"))
  (if (`self.ActorHasTag` OtherActor "Piso")
    (set `self.PuedeSaltar` true)))

(fn `UserConstructionScript`)