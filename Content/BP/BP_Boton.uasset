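; BP_Boton is a button that reacts to BP_Character stepping on or off its Plane trigger.
; Begin and end overlap each play a separate timeline that drives the Cube's relative Z.
; Each timeline update also sets the character's BotonApretado flag, true on entry and false on exit.
; Both timelines use Play rather than PlayFromStart, so neither rewinds between overlaps.
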(event `self.Plane.OnComponentBeginOverlap`
  (params (OverlappedComponent :type "PrimitiveComponent Object Reference") (OtherActor :type "Actor Object Reference") (OtherComp :type "PrimitiveComponent Object Reference") (OtherBodyIndex :type Integer) (bFromSweep :type Boolean) (SweepResult :type "HitResult Structure (by ref)"))
  (bind _asbp_character (cast `/Game/BP/BP_Character` OtherActor))
  (bind (_direction _newtrack_0) (`Timeline|Línea de tiempo_1`)
    (:`Update`
      (`SceneComponent.K2_SetRelativeLocation` (`self.Cube`) (`KismetMathLibrary.MakeVector` 0.0 0.0 _newtrack_0) false false)
      (set `/Game/BP/BP_Character.BotonApretado` true _asbp_character))))

(event `self.Plane.OnComponentEndOverlap`
  (params (OverlappedComponent :type "PrimitiveComponent Object Reference") (OtherActor :type "Actor Object Reference") (OtherComp :type "PrimitiveComponent Object Reference") (OtherBodyIndex :type Integer))
  (bind _asbp_character (cast `/Game/BP/BP_Character` OtherActor))
  (bind (_direction _newtrack_0) (`Timeline|Línea de tiempo_0`)
    (:`Update`
      (`SceneComponent.K2_SetRelativeLocation` (`self.Cube`) (`KismetMathLibrary.MakeVector` 0.0 0.0 _newtrack_0) false false)
      (set `/Game/BP/BP_Character.BotonApretado` false _asbp_character))))

(fn `UserConstructionScript`)