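; BP_Enemigo2 is a moving enemy that pushes the player character away on contact.
; From BeginPlay, a Timeline offsets the actor from its starting location without sweeping.
; When its Cube hits a BP_Character, a RadialForce component activates briefly, then switches off.
; Logic to subtract a life (Vidas) from BP_Gamemode through a DoOnce is present but disconnected, so it never runs.
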(event `self.ReceiveActorBeginOverlap`
  (params (OtherActor :type "Actor Object Reference")))

(event `self.ReceiveBeginPlay`
  (set `self.Posicion` (`self.K2_GetActorLocation`))
  (bind (_direction _newtrack_0) (`Timeline|Timeline_2`)
    (:`Update`
      (`self.K2_SetActorLocation` (+ (`self.Posicion`) _newtrack_0)))))

(event `self.Cube.OnComponentHit`
  (params (HitComponent :type "PrimitiveComponent Object Reference") (OtherActor :type "Actor Object Reference") (OtherComp :type "PrimitiveComponent Object Reference") (NormalImpulse :type "Vector Structure") (Hit :type "HitResult Structure (by ref)"))
  (cast `/Game/BP/BP_Character` OtherActor)
  (`ActorComponent.Activate` (`self.RadialForce`) false)
  (`KismetSystemLibrary.Delay` 0.2)
  (`ActorComponent.Deactivate` (`self.RadialForce`)))

(fn `UserConstructionScript`)